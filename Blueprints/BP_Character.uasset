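; Character Blueprint that plays a physical hit reaction on the HeadHit1 mesh, ignoring Hips hits and new hits during a reaction.
; A timeline drives BlendWeight, which Tick applies as physics simulation and blend weight to the hit bone and those below it.
; After a brief delay, an impulse along the camera's forward direction kicks the bone.
; When the timeline finishes, physics is switched off.
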(event Custom|HitReaction
  (params (Bone :type Name) (hit%20location :type Vector))
  (bind _head_hit__1_ (Variables|PhysicsAnimation|GetHead_Hit__1_))
  (if (!= Bone "Hips")
    (if (not (Variables|Default|GetIs%20Hit))
      (Variables|Default|SetIs%20Hit true)
      (Variables|Default|SetBoneName Bone)
      (Utilities|FlowControl|Sequence
        (:then_0
          (bind _新建轨道_0 (Timeline|时间轴_0 PlayFromStart)
            (:Update
              (Variables|Default|SetBlendWeight _新建轨道_0))
            (:Finished
              (Class|SkeletalMeshComponent|SetAllBodiesPhysicsBlendWeight _head_hit__1_ 0.0 false)
              (Class|SkeletalMeshComponent|SetAllBodiesSimulatePhysics _head_hit__1_ false)
              (Variables|Default|SetIs%20Hit false))))
        (:then_1
          (Utilities|FlowControl|Delay 0.048)
          (Physics|AddImpulse (Variables|PhysicsAnimation|GetHead_Hit__1_) (* (Math|Vector|GetForwardVector (Transformation|GetActorRotation (Game|GetPlayerCameraManager 0))) 1.2e+03) (Variables|Default|GetBoneName) true))))))

(event EventTick
  (params (DeltaSeconds :type Float%20%28single-precision%29))
  (bind _head_hit__1_ (Variables|PhysicsAnimation|GetHead_Hit__1_))
  (bind _bonename (Variables|Default|GetBoneName))
  (if (> (Variables|Default|GetBlendWeight) 0.0)
    (Class|SkeletalMeshComponent|SetAllBodiesBelowSimulatePhysics _head_hit__1_ _bonename true true)
    (Class|SkeletalMeshComponent|SetAllBodiesBelowPhysicsBlendWeight _head_hit__1_ _bonename (Variables|Default|GetBlendWeight) false true)))

(fn ConstructionScript)